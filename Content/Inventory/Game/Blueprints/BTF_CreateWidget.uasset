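; Blueprint function library that builds the in-game inventory UI at runtime.
; CreateWidgetMain adds the master widget to the viewport, then populates equipment, bag and chest slots, tabs, item tooltip rows and character stat panels, registering widget references in the game instance and inventory.
; A shared slot loop switches on container type; a separate function builds the shop grid.
; Craft list creation, craft tooltip rows and skill/flask slot creation are disconnected.
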(fn `CreateWidget_BagTab`
  (bind _asmy_game_instance (cast `/Game/Game/MyGameInstance` (`GameplayStatics.GetGameInstance` null)))
  (bind _returnvalue (`|CreateWidget` "/Game/Game/Widget/Inventory/W_BagTabButton.W_BagTabButton_C"))
  (`PanelWidget.AddChild` (`/Game/Game/Widget/Inventory/W_InventroryBag.HorizontalBox_StashBag` (`/Game/Game/Widget/W_MasterInGame.W_InventroryBag` (`/Game/Game/MyGameInstance.Ref_WidgetMasterInGame` _asmy_game_instance))) _returnvalue)
  (bind _ref_inventory (`/Game/Game/MyGameInstance.Ref_Inventory` _asmy_game_instance))
  (bind _returnvalue_2 (+ (`KismetArrayLibrary.Array_LastIndex` (`/Game/Game/Inventory/Bp_Inventory.ItemInBagArray` _ref_inventory)) 1))
  (set `/Game/Game/Widget/Inventory/W_BagTabButton.IndexButton` _returnvalue_2 _returnvalue)
  (set `/Game/Game/Widget/Inventory/W_BagTabButton.Ref_Inventory` _ref_inventory _returnvalue)
  (`KismetArrayLibrary.Array_Add` (`/Game/Game/Inventory/Bp_Inventory.ItemInBagArray` _ref_inventory))
  (`TextBlock.SetText` (`/Game/Game/Widget/Inventory/W_BagTabButton.BagTabName` _returnvalue) (`KismetTextLibrary.Conv_StringToText` (`KismetStringLibrary.Concat_StrStr` "Tab " (`KismetStringLibrary.Conv_IntToString` _returnvalue_2))))
  (`/Engine/EditorBlueprintResources/StandardMacros.IsValid` (`/Game/Game/Inventory/Bp_Inventory.LastBagStashTab` _ref_inventory)
    (:`Is Not Valid`
      ;[0.1177 0.1177 0.1177] Add First ref Bag Tab
      (set `/Game/Game/Inventory/Bp_Inventory.LastBagStashTab` _returnvalue _ref_inventory)
      (`Button.SetBackgroundColor` (`/Game/Game/Widget/Inventory/W_BagTabButton.Button_SelectChest` _returnvalue) (struct :`R` 1.0 :`G` 1.0 :`B` 1.0 :`A` 1.0)))))

(fn `CreateWidget_CharStat`
  (params (MyGameInstance :type "/Game/Game/MyGameInstance Object Reference"))
  (locals (Ref_MyGameInstance :type "/Game/Game/MyGameInstance Object Reference") (Ref_CharStatDefence :type "Array of /Game/Game/Widget/CharStat/W_CharStatSingleStat Object Reference"))
  (set `local.Ref_MyGameInstance` MyGameInstance)
  (`KismetArrayLibrary.Array_Clear` (`/Game/Game/MyGameInstance.Ref_CharStatOffence` (`local.Ref_MyGameInstance`)))
  (`KismetArrayLibrary.Array_Clear` (`/Game/Game/MyGameInstance.Ref_CharStatDefence` (`local.Ref_MyGameInstance`)))
  (bind _returnvalue (`|CreateWidget` "/Game/Game/Widget/CharStat/W_CharStatSpawnStat.W_CharStatSpawnStat_C"))
  (`PanelWidget.AddChild` (`/Game/Game/Widget/CharStat/W_CharStat.WidgetSwitcher_ShowStat` (`/Game/Game/Widget/W_MasterInGame.W_CharStat` (`/Game/Game/MyGameInstance.Ref_WidgetMasterInGame` (`local.Ref_MyGameInstance`)))) _returnvalue)
  (for _index (range 14)
    (bind _returnvalue_2 (`|CreateWidget` "/Game/Game/Widget/CharStat/W_CharStatSingleStat.W_CharStatSingleStat_C"))
    (`KismetArrayLibrary.Array_Add` (`/Game/Game/MyGameInstance.Ref_CharStatOffence` (`local.Ref_MyGameInstance`)) _returnvalue_2)
    (`PanelWidget.AddChild` (`/Game/Game/Widget/CharStat/W_CharStatSpawnStat.VerticalBox_SpawnStat` _returnvalue) _returnvalue_2)
    (`Widget.SetVisibility` (`/Game/Game/Widget/CharStat/W_CharStatSingleStat.TextBlock_StatPercent` _returnvalue_2) (select `int` _index :`0` "Visible" :`1` "Visible" :`2` "Hidden" :`3` "Hidden" :`4` "Hidden" :`5` "Hidden" :`6` "Hidden" :`7` "Visible" :`8` "Visible" :`9` "Hidden" :`10` "Visible" :`11` "Visible" :`12` "Hidden" :`13` "Hidden" :!type "ESlateVisibility Enum"))
    (`/Engine/EditorBlueprintResources/StandardMacros.FlipFlop`
      (:`B`
        (`Border.SetBrushColor` (`/Game/Game/Widget/CharStat/W_CharStatSingleStat.Border_0` _returnvalue_2) (struct :`R` 0.015625 :`G` 0.015625 :`B` 0.015625 :`A` 1.0)))))
  (bind _returnvalue_3 (`|CreateWidget` "/Game/Game/Widget/CharStat/W_CharStatSpawnStat.W_CharStatSpawnStat_C"))
  (`PanelWidget.AddChild` (`/Game/Game/Widget/CharStat/W_CharStat.WidgetSwitcher_ShowStat` (`/Game/Game/Widget/W_MasterInGame.W_CharStat` (`/Game/Game/MyGameInstance.Ref_WidgetMasterInGame` (`local.Ref_MyGameInstance`)))) _returnvalue_3)
  (for _index_2 (range 14)
    (bind _returnvalue_4 (`|CreateWidget` "/Game/Game/Widget/CharStat/W_CharStatSingleStat.W_CharStatSingleStat_C"))
    (`KismetArrayLibrary.Array_Add` (`/Game/Game/MyGameInstance.Ref_CharStatDefence` (`local.Ref_MyGameInstance`)) _returnvalue_4)
    (`PanelWidget.AddChild` (`/Game/Game/Widget/CharStat/W_CharStatSpawnStat.VerticalBox_SpawnStat` _returnvalue_3) _returnvalue_4)
    (`Widget.SetVisibility` (`/Game/Game/Widget/CharStat/W_CharStatSingleStat.TextBlock_StatPercent` _returnvalue_4) (select `int` _index_2 :`0` "Hidden" :`1` "Visible" :`2` "Visible" :`3` "Visible" :`4` "Visible" :`5` "Visible" :`6` "Visible" :`7` "Visible" :`8` "Visible" :`9` "Visible" :`10` "Visible" :`11` "Hidden" :`12` "Hidden" :`13` "Hidden" :!type "ESlateVisibility Enum"))
    (`/Engine/EditorBlueprintResources/StandardMacros.FlipFlop`
      (:`B`
        (`Border.SetBrushColor` (`/Game/Game/Widget/CharStat/W_CharStatSingleStat.Border_0` _returnvalue_4) (struct :`R` 0.015625 :`G` 0.015625 :`B` 0.015625 :`A` 1.0))))))

(fn `CreateWidget_CharStatStrDexInt`
  (params (MyGameInstance :type "/Game/Game/MyGameInstance Object Reference"))
  (locals (Ref_MyGameInstance :type "/Game/Game/MyGameInstance Object Reference") (Ref_CharStatDefence :type "Array of /Game/Game/Widget/CharStat/W_CharStatSingleStat Object Reference"))
  (bind _w_charstat (`/Game/Game/Widget/W_MasterInGame.W_CharStat` (`/Game/Game/MyGameInstance.Ref_WidgetMasterInGame` (`local.Ref_MyGameInstance`))))
  (set `local.Ref_MyGameInstance` MyGameInstance)
  (`KismetArrayLibrary.Array_Clear` (`/Game/Game/MyGameInstance.Ref_CharStatStatStrDexInt1` (`local.Ref_MyGameInstance`)))
  (for _index (range 6)
    (bind _returnvalue (`|CreateWidget` "/Game/Game/Widget/CharStat/W_CharStatStrDexInt.W_CharStatStrDexInt_C"))
    (`KismetArrayLibrary.Array_Add` (`/Game/Game/MyGameInstance.Ref_CharStatStatStrDexInt1` (`local.Ref_MyGameInstance`)) _returnvalue)
    (set `/Game/Game/Widget/CharStat/W_CharStatStrDexInt.IndexStat` _index _returnvalue)
    (set `/Game/Game/Widget/CharStat/W_CharStatStrDexInt.Ref_Inventory` (`/Game/Game/MyGameInstance.Ref_Inventory` (`local.Ref_MyGameInstance`)) _returnvalue)
    (`/Engine/EditorBlueprintResources/StandardMacros.FlipFlop`
      (:`A`
        (`PanelWidget.AddChild` (`/Game/Game/Widget/CharStat/W_CharStat.VerticalBox_StrDexInt` _w_charstat) _returnvalue))
      (:`B`
        (`PanelWidget.AddChild` (`/Game/Game/Widget/CharStat/W_CharStat.VerticalBox_VitLuckWill` _w_charstat) _returnvalue)))))

(fn `CreateWidget_ChestTab`
  (bind _asmy_game_instance (cast `/Game/Game/MyGameInstance` (`GameplayStatics.GetGameInstance` null)))
  (bind _returnvalue (`|CreateWidget` "/Game/Game/Widget/Chest/W_ChestSingleSwitchButton.W_ChestSingleSwitchButton_C"))
  (`PanelWidget.AddChild` (`/Game/Game/Widget/Chest/W_Chest.ScrollBox_SelectChestSpawnButton` (`/Game/Game/Widget/W_MasterInGame.W_Chest` (`/Game/Game/MyGameInstance.Ref_WidgetMasterInGame` _asmy_game_instance))) _returnvalue)
  (bind _ref_inventory (`/Game/Game/MyGameInstance.Ref_Inventory` _asmy_game_instance))
  (bind _returnvalue_2 (+ (`KismetArrayLibrary.Array_LastIndex` (`/Game/Game/Inventory/Bp_Inventory.ItemInChest` _ref_inventory)) 1))
  (set `/Game/Game/Widget/Chest/W_ChestSingleSwitchButton.IndexButton` _returnvalue_2 _returnvalue)
  (set `/Game/Game/Widget/Chest/W_ChestSingleSwitchButton.Ref_Inventory` _ref_inventory _returnvalue)
  (`KismetArrayLibrary.Array_Add` (`/Game/Game/Inventory/Bp_Inventory.ItemInChest` _ref_inventory))
  (`TextBlock.SetText` (`/Game/Game/Widget/Chest/W_ChestSingleSwitchButton.ChestName` _returnvalue) (`KismetTextLibrary.Conv_StringToText` (`KismetStringLibrary.Concat_StrStr` "Tab " (`KismetStringLibrary.Conv_IntToString` _returnvalue_2))))
  (`/Engine/EditorBlueprintResources/StandardMacros.IsValid` (`/Game/Game/Inventory/Bp_Inventory.LastChestStashTab` _ref_inventory)
    (:`Is Not Valid`
      ;[0.1177 0.1177 0.1177] Add First ref Bag Tab
      (set `/Game/Game/Inventory/Bp_Inventory.LastChestStashTab` _returnvalue _ref_inventory)
      (`Border.SetBrushColor` (`/Game/Game/Widget/Chest/W_ChestSingleSwitchButton.Border_SelectButton` _returnvalue) (struct :`R` 0.71875 :`G` 0.71875 :`B` 0.71875 :`A` 1.0)))))

(fn `CreateWidget_CraftItemList`
  (params (Ref_MyGameInstance :type "/Game/Game/MyGameInstance Object Reference")))

(fn `CreateWidget_CreateInventorySlot`
  (params (MyGameInstance :type "/Game/Game/MyGameInstance Object Reference"))
  (locals (FirstIndex :type Integer) (LastIndex :type Integer) (Switch :type Integer) (Ref_GridPanel :type "UniformGridPanel Object Reference") (Column :type Integer) (Row :type Integer) (Ref_WMasterInGame :type "/Game/Game/Widget/W_MasterInGame Object Reference") (IndexLoop1 :type Integer) (Ref_WSingleSlot :type "/Game/Game/Widget/Inventory/W_InventrorySingleSlot Object Reference") (Ref_WSingleSlotArray :type "Array of /Game/Game/Widget/Inventory/W_InventrorySingleSlot Object Reference") (Ref_Inventory :type "/Game/Game/Inventory/Bp_Inventory Object Reference") (IndexItemInSlotBag1 :type "Array of Integer") (ChestHowManySlot :type Integer) (Ref_ButtonChesSlot :type "Array of /Game/Game/Widget/Chest/W_ChestSingleSwitchButton Object Reference") (Ref_MyGameInstance :type "/Game/Game/MyGameInstance Object Reference"))
  (bind _indexloop1 (`local.IndexLoop1`))
  (bind _ref_wsingleslot (`local.Ref_WSingleSlot`))
  (bind _ref_inventory (`local.Ref_Inventory`))
  (bind _w_inventroyequipmentitem (`/Game/Game/Widget/W_MasterInGame.W_InventroyEquipmentItem` (`local.Ref_WMasterInGame`)))
  ;[1 0 0] Old For change
  (set `local.Ref_MyGameInstance` MyGameInstance)
  (set `local.Ref_WMasterInGame` (`/Game/Game/MyGameInstance.Ref_WidgetMasterInGame` (`local.Ref_MyGameInstance`)))
  (set `local.Ref_Inventory` (`/Game/Game/MyGameInstance.Ref_Inventory` (`local.Ref_MyGameInstance`)))
  (`|ExecutionSequence`
    (:`then_0`
      ;;[1 1 1] Equipment --- 19 Slot
      (set `local.FirstIndex` 0)
      (set `local.LastIndex` 19)
      (set `local.Switch` 0)
      (set `/Game/Game/Widget/Inventory/W_InventroyEquipmentItem.Ref_Inventory` (`local.Ref_Inventory`) (`/Game/Game/Widget/W_MasterInGame.W_InventroyEquipmentItem` (`local.Ref_WMasterInGame`)))
      (for _index (range (`local.FirstIndex`) (+ (`local.LastIndex`) 1)) :!label _label
        (set `local.IndexLoop1` _index)
        (bind _returnvalue (`|CreateWidget` "/Game/Game/Widget/Inventory/W_InventrorySingleSlot.W_InventrorySingleSlot_C"))
        (set `local.Ref_WSingleSlot` _returnvalue)
        (set `/Game/Game/Widget/Inventory/W_InventrorySingleSlot.IndexSlot` (`local.IndexLoop1`) (`local.Ref_WSingleSlot`))
        (set `/Game/Game/Widget/Inventory/W_InventrorySingleSlot.Ref_Inventory` _ref_inventory (`local.Ref_WSingleSlot`))
        (`KismetArrayLibrary.Array_Add` (`local.IndexItemInSlotBag1`) -1)
        (switch `int` (`local.Switch`)
          (:`0`
            (`KismetArrayLibrary.Array_Add` (`/Game/Game/Inventory/Bp_Inventory.IndexItemInEquipment` _ref_inventory) -1)
            (`KismetArrayLibrary.Array_Add` (`/Game/Game/Inventory/Bp_Inventory.RefWidgetEquipment` _ref_inventory) (`local.Ref_WSingleSlot`))
            (set `/Game/Game/Widget/Inventory/W_InventrorySingleSlot.TypeSlot` "NewEnumerator4" (`local.Ref_WSingleSlot`))
            ;[1 1 1] Create Equpmnet slot
            ;;[1 1 1] Skip Equipment Empty Slot
            (if (not (or (== _indexloop1 3) (== _indexloop1 14) (== _indexloop1 15) (== _indexloop1 0)))
              (bind _returnvalue_2 (`|CreateWidget` "/Game/Game/Widget/Inventory/W_MouseOutInSlot.W_MouseOutInSlot_C"))
              (set `/Game/Game/Widget/Inventory/W_MouseOutInSlot.Ref_Inventory` (`local.Ref_Inventory`) _returnvalue_2)
              (`PanelWidget.AddChild` (select `int` (`local.IndexLoop1`) :`0` null :`1` (`/Game/Game/Widget/Inventory/W_InventroyEquipmentItem.01_Helm` _w_inventroyequipmentitem) :`2` (`/Game/Game/Widget/Inventory/W_InventroyEquipmentItem.02_Armor` _w_inventroyequipmentitem) :`3` null :`4` (`/Game/Game/Widget/Inventory/W_InventroyEquipmentItem.04_Pas` _w_inventroyequipmentitem) :`5` (`/Game/Game/Widget/Inventory/W_InventroyEquipmentItem.05_Gloves` _w_inventroyequipmentitem) :`6` (`/Game/Game/Widget/Inventory/W_InventroyEquipmentItem.06_Pants` _w_inventroyequipmentitem) :`7` (`/Game/Game/Widget/Inventory/W_InventroyEquipmentItem.07_Boots` _w_inventroyequipmentitem) :`8` (`/Game/Game/Widget/Inventory/W_InventroyEquipmentItem.8_Amulet` _w_inventroyequipmentitem) :`9` (`/Game/Game/Widget/Inventory/W_InventroyEquipmentItem.9_Itemxxx` _w_inventroyequipmentitem) :`10` (`/Game/Game/Widget/Inventory/W_InventroyEquipmentItem.10_RingLeft2` _w_inventroyequipmentitem) :`11` (`/Game/Game/Widget/Inventory/W_InventroyEquipmentItem.11_RingLeft1` _w_inventroyequipmentitem) :`12` (`/Game/Game/Widget/Inventory/W_InventroyEquipmentItem.12_RingRights2` _w_inventroyequipmentitem) :`13` (`/Game/Game/Widget/Inventory/W_InventroyEquipmentItem.13_RingRights1` _w_inventroyequipmentitem) :`14` null :`15` null :`16` (`/Game/Game/Widget/Inventory/W_InventroyEquipmentItem.16_WeaponLeft` _w_inventroyequipmentitem) :`17` (`/Game/Game/Widget/Inventory/W_InventroyEquipmentItem.17_WeaponRightOrShield` _w_inventroyequipmentitem) :`18` (`/Game/Game/Widget/Inventory/W_InventroyEquipmentItem.18_WeaponLeft` _w_inventroyequipmentitem) :`19` (`/Game/Game/Widget/Inventory/W_InventroyEquipmentItem.19_WeaponRightOrShield` _w_inventroyequipmentitem)) _returnvalue_2)
              (`PanelWidget.AddChild` (`/Game/Game/Widget/Inventory/W_MouseOutInSlot.Border_0` _returnvalue_2) _ref_wsingleslot)
              (`Widget.SetVisibility` (`/Game/Game/Widget/Inventory/W_InventrorySingleSlot.Image_SingleSlot` _ref_wsingleslot) "Hidden")))
          (:`3`
            (`KismetArrayLibrary.Array_Add` (`/Game/Game/Inventory/Bp_Inventory.IndexItemInChest` _ref_inventory) -1)
            (`KismetArrayLibrary.Array_Add` (`/Game/Game/Inventory/Bp_Inventory.RefWidgetChest` _ref_inventory) (`local.Ref_WSingleSlot`))
            (set `/Game/Game/Widget/Inventory/W_InventrorySingleSlot.TypeSlot` "NewEnumerator2" (`local.Ref_WSingleSlot`))
            ;[1 1 1] Create Bag Slot
            (set `local.Column` (+ (`local.Column`) 1) :!label _label_2)
            (if (== (`local.Column`) 10)
              (set `local.Column` 0)
              (set `local.Row` (+ (`local.Row`) 1)))
            (bind _returnvalue_3 (`UniformGridPanel.AddChildToUniformGrid` (`local.Ref_GridPanel`) (`local.Ref_WSingleSlot`)))
            (`UniformGridSlot.SetColumn` _returnvalue_3 (`local.Column`))
            (`UniformGridSlot.SetRow` _returnvalue_3 (`local.Row`)))
          (:`4`
            (`KismetArrayLibrary.Array_Add` (`/Game/Game/Inventory/Bp_Inventory.IndexItemInBag` _ref_inventory) -1)
            (`KismetArrayLibrary.Array_Add` (`/Game/Game/Inventory/Bp_Inventory.RefWidgetBag` _ref_inventory) (`local.Ref_WSingleSlot`))
            (set `/Game/Game/Widget/Inventory/W_InventrorySingleSlot.TypeSlot` "NewEnumerator1" (`local.Ref_WSingleSlot`))
            (goto _label_2)))))
    (:`then_1`
      ;;[1 1 1] Skill Slot --- 45 Slot
      (set `local.FirstIndex` 20)
      (set `local.LastIndex` 65)
      (set `local.Switch` 1))
    (:`then_2`
      ;;[1 1 1] Flask Slot  --- 4 Slot
      (set `local.FirstIndex` 66)
      (set `local.LastIndex` 69)
      (set `local.Switch` 2))
    (:`then_3`
      ;;[1 1 1] Bag Slot  --- 79 Slot // 139 // 153
      (set `local.FirstIndex` 0)
      (set `local.LastIndex` 69)
      (set `local.Switch` 4)
      (set `local.Ref_GridPanel` (`/Game/Game/Widget/Inventory/W_UniformGridPanel.UniformGridPanel_0` (`/Game/Game/Widget/Inventory/W_InventroryBag.W_UniformGridPanel` (`/Game/Game/Widget/W_MasterInGame.W_InventroryBag` (`local.Ref_WMasterInGame`)))))
      (set `local.Column` -1)
      (set `local.Row` 0)
      (`|ExecutionSequence`
        (:`then_0`
          (goto _label))))
    (:`then_4`
      ;;[1 1 1] Chest Slot  --- 164 hmm Slot
      (set `local.ChestHowManySlot` 0)
      (set `local.FirstIndex` 0)
      (set `local.LastIndex` 139)
      (set `local.Switch` 3)
      (set `local.Column` -1)
      (set `local.Row` 0)
      (bind _returnvalue_4 (`|CreateWidget` "/Game/Game/Widget/Inventory/W_UniformGridPanel.W_UniformGridPanel_C"))
      (set `local.Ref_GridPanel` (`/Game/Game/Widget/Inventory/W_UniformGridPanel.UniformGridPanel_0` _returnvalue_4))
      (`PanelWidget.AddChild` (`/Game/Game/Widget/Chest/W_ChestSpawnSlot.VerticalBox_SpawnChest` (`/Game/Game/Widget/Chest/W_Chest.W_ChestSpawnSlot` (`/Game/Game/Widget/W_MasterInGame.W_Chest` (`local.Ref_WMasterInGame`)))) (`local.Ref_GridPanel`))
      (set `/Game/Game/Widget/Chest/W_ChestSpawnSlot.Ref_Inventory` (`local.Ref_Inventory`) (`/Game/Game/Widget/Chest/W_Chest.W_ChestSpawnSlot` (`/Game/Game/Widget/W_MasterInGame.W_Chest` (`local.Ref_WMasterInGame`))))
      (goto _label))
    (:`then_5`
      ;;[1 1 1] Set To My Game Instance
      (set `/Game/Game/MyGameInstance.Ref_WSingleSlotArray` (`local.Ref_WSingleSlotArray`) (`local.Ref_MyGameInstance`))
      ;;[1 1 1] Set To Bp Inventory
      (set `/Game/Game/Inventory/Bp_Inventory.IndexItemInSlotBag1` (`local.IndexItemInSlotBag1`) (`local.Ref_Inventory`))
      (set `/Game/Game/Widget/Inventory/W_InventroryBag.Ref_Inventory` (`local.Ref_Inventory`) (`/Game/Game/Widget/W_MasterInGame.W_InventroryBag` (`local.Ref_WMasterInGame`)))
      (set `/Game/Game/Inventory/Bp_Inventory.Ref_ButtonChesSlot1` (`local.Ref_ButtonChesSlot`) (`local.Ref_Inventory`)))))

(fn `CreateWidget_Main`
  (params (MyGameInstance :type "/Game/Game/MyGameInstance Object Reference"))
  (locals (Ref_MyGameInstance :type "/Game/Game/MyGameInstance Object Reference"))
  (set `local.Ref_MyGameInstance` MyGameInstance)
  (bind _returnvalue (`|CreateWidget` "/Game/Game/Widget/W_MasterInGame.W_MasterInGame_C"))
  (`UserWidget.AddToViewport` _returnvalue 0)
  (set `/Game/Game/MyGameInstance.Ref_WidgetMasterInGame` _returnvalue (`local.Ref_MyGameInstance`))
  (`|ExecutionSequence`
    (:`then_0`
      (`self.CreateWidget_CreateInventorySlot` (`local.Ref_MyGameInstance`)))
    (:`then_1`
      (for _ (range 3)
        (`self.CreateWidget_BagTab` null)))
    (:`then_2`
      (for _ (range 3)
        (`self.CreateWidget_ChestTab` null)))
    (:`then_4`
      (`self.CreateWidget_ShowItemStat` (`local.Ref_MyGameInstance`)))
    (:`then_5`
      (`self.CreateWidget_CraftItemList` (`local.Ref_MyGameInstance`)))
    (:`then_6`
      (`self.CreateWidget_CharStatStrDexInt` (`local.Ref_MyGameInstance`)))
    (:`then_7`
      (`self.CreateWidget_SelectCharStat` (`local.Ref_MyGameInstance`)))
    (:`then_8`
      (`self.CreateWidget_CharStat` (`local.Ref_MyGameInstance`)))))

(fn `CreateWidget_SelectCharStat`
  (params (MyGameInstance :type "/Game/Game/MyGameInstance Object Reference"))
  (locals (Ref_MyGameInstance :type "/Game/Game/MyGameInstance Object Reference") (Ref_CharStatButton :type "/Game/Game/Widget/CharStat/W_CharStatSelectStatSingleButton Object Reference"))
  (bind _w_charstat (`/Game/Game/Widget/W_MasterInGame.W_CharStat` (`/Game/Game/MyGameInstance.Ref_WidgetMasterInGame` (`local.Ref_MyGameInstance`))))
  (set `local.Ref_MyGameInstance` MyGameInstance)
  (for _index (range 2)
    (bind _returnvalue (`|CreateWidget` "/Game/Game/Widget/CharStat/W_CharStatSelectStatSingleButton.W_CharStatSelectStatSingleButton_C"))
    (set `local.Ref_CharStatButton` _returnvalue)
    (`PanelWidget.AddChild` (`/Game/Game/Widget/CharStat/W_CharStat.ScrollBox_CharStat` _w_charstat) (`local.Ref_CharStatButton`))
    (set `/Game/Game/Widget/CharStat/W_CharStatSelectStatSingleButton.IndexButtonCharStat` _index (`local.Ref_CharStatButton`))
    (set `/Game/Game/Widget/CharStat/W_CharStatSelectStatSingleButton.Ref_CharStat` _w_charstat (`local.Ref_CharStatButton`))
    (`Image.SetBrushFromTexture` (`/Game/Game/Widget/CharStat/W_CharStatSelectStatSingleButton.Image_0` (`local.Ref_CharStatButton`)) (select `int` _index :`0` "/Game/Game/Widget/IconTest/SelectStatOffence.SelectStatOffence" :`1` "/Game/Game/Widget/IconTest/SelectStatDefence.SelectStatDefence" :`2` null :!type "Texture2D Object Reference") false)))

(fn `CreateWidget_Shop`
  (params (Ref_MyGameInstance :type "/Game/Game/MyGameInstance Object Reference") (Ref_widgetShop :type "/Game/Game/Widget/Shop/W_Shop Object Reference"))
  (locals (Ref_Inventory :type "/Game/Game/Inventory/Bp_Inventory Object Reference") (Ref_Shop :type "/Game/Game/Widget/Shop/W_Shop Object Reference") (Column :type Integer) (Row :type Integer) (Ref_WSingleSlotArray :type "Array of /Game/Game/Widget/Inventory/W_InventrorySingleSlot Object Reference") (IndexItemInSlotBag1 :type "Array of Integer") (Ref_GridPanel :type "UniformGridPanel Object Reference"))
  (set `local.Ref_Shop` Ref_widgetShop)
  (set `local.Ref_Inventory` (`/Game/Game/MyGameInstance.Ref_Inventory` Ref_MyGameInstance))
  ;[1 1 1] Chest Slot  --- 164 hmm Slot
  (set `local.Column` -1)
  (set `local.Row` 0)
  (bind _returnvalue (`|CreateWidget` "/Game/Game/Widget/Inventory/W_UniformGridPanel.W_UniformGridPanel_C"))
  (bind _output_get (set `local.Ref_GridPanel` (`/Game/Game/Widget/Inventory/W_UniformGridPanel.UniformGridPanel_0` _returnvalue)))
  (`PanelWidget.AddChild` (`/Game/Game/Widget/Chest/W_ChestSpawnSlot.VerticalBox_SpawnChest` (`/Game/Game/Widget/Shop/W_Shop.W_ChestSwither` (`local.Ref_Shop`))) _output_get)
  (for _index (range 1 166)
    (bind _returnvalue_2 (`|CreateWidget` "/Game/Game/Widget/Inventory/W_InventrorySingleSlot.W_InventrorySingleSlot_C"))
    (`KismetArrayLibrary.Array_Add` (`local.Ref_WSingleSlotArray`) _returnvalue_2)
    (set `/Game/Game/Widget/Inventory/W_InventrorySingleSlot.IndexSlot` _index _returnvalue_2)
    (set `/Game/Game/Widget/Inventory/W_InventrorySingleSlot.Ref_Inventory` (`local.Ref_Inventory`) _returnvalue_2)
    (`KismetArrayLibrary.Array_Add` (`local.IndexItemInSlotBag1`) -1)
    ;[1 1 1] Create Bag Slot
    (set `local.Column` (+ (`local.Column`) 1))
    (if (== (`local.Column`) 11)
      (set `local.Column` 0)
      (set `local.Row` (+ (`local.Row`) 1)))
    (bind _returnvalue_3 (`UniformGridPanel.AddChildToUniformGrid` (`local.Ref_GridPanel`) _returnvalue_2))
    (`UniformGridSlot.SetColumn` _returnvalue_3 (`local.Column`))
    (`UniformGridSlot.SetRow` _returnvalue_3 (`local.Row`))))

(fn `CreateWidget_ShowItemStat`
  (params (MyGameInstance :type "/Game/Game/MyGameInstance Object Reference"))
  (locals (Ref_MyGameInstance :type "/Game/Game/MyGameInstance Object Reference") (Ref_WMasterInGame :type "/Game/Game/Widget/W_MasterInGame Object Reference") (Ref_ItemInfo :type "/Game/Game/Widget/Inventory/W_InventoryItemInfo Object Reference") (ItemInfoOrCraft :type Boolean) (IndexLoop1 :type Integer) (Ref_ItemInfoSingleStat :type "/Game/Game/Widget/Inventory/W_InventoryItemInfoSingleStat Object Reference") (Ref_Inventory :type "/Game/Game/Inventory/Bp_Inventory Object Reference") (Ref_ItemInfo_NameAndRequrmest :type "Array of /Game/Game/Widget/Inventory/W_InventoryItemInfoSingleStat Object Reference") (Ref_ItemInfo_MainStat :type "Array of /Game/Game/Widget/Inventory/W_InventoryItemInfoSingleStat Object Reference") (Ref_ItemInfo_SecondStat :type "Array of /Game/Game/Widget/Inventory/W_InventoryItemInfoSingleStat Object Reference") (Ref_Craft_ItemInfo_NameAndRequrmest :type "Array of /Game/Game/Widget/Inventory/W_InventoryItemInfoSingleStat Object Reference") (Ref_Craft_ItemInfo_MainStat :type "Array of /Game/Game/Widget/Inventory/W_InventoryItemInfoSingleStat Object Reference") (Ref_Craft_ItemInfo_SecondStat :type "Array of /Game/Game/Widget/Inventory/W_InventoryItemInfoSingleStat Object Reference") (IndexLoop :type Integer))
  (bind _ref_iteminfosinglestat (`local.Ref_ItemInfoSingleStat`))
  (bind _textblock_statvalue (`/Game/Game/Widget/Inventory/W_InventoryItemInfoSingleStat.TextBlock_StatValue` (`local.Ref_ItemInfoSingleStat`)))
  (bind _textblock_statname (`/Game/Game/Widget/Inventory/W_InventoryItemInfoSingleStat.TextBlock_StatName` (`local.Ref_ItemInfoSingleStat`)))
  (bind _textblock_statvalue_2 (`/Game/Game/Widget/Inventory/W_InventoryItemInfoSingleStat.TextBlock_StatValue` _ref_iteminfosinglestat))
  (bind _textblock_statname_2 (`/Game/Game/Widget/Inventory/W_InventoryItemInfoSingleStat.TextBlock_StatName` _ref_iteminfosinglestat))
  (bind (_font_fontobject _font_fontmaterial _font_outlinesettings) (break `SlateFontInfo` (`TextBlock.Font` _textblock_statname)))
  (bind (_font_fontobject_2 _font_fontmaterial_2 _font_outlinesettings_2 _font_typefacefontname) (break `SlateFontInfo` (`TextBlock.Font` _textblock_statname_2)))
  (bind (_font_fontobject_3 _font_fontmaterial_3 _font_outlinesettings_3) (break `SlateFontInfo` (`TextBlock.Font` _textblock_statvalue)))
  (bind (_font_fontobject_4 _font_fontmaterial_4 _font_outlinesettings_4 _font_typefacefontname_2) (break `SlateFontInfo` (`TextBlock.Font` _textblock_statvalue_2)))
  ;[1 1 1] Widget Show Item Stat
  (bind _output_get (set `local.Ref_MyGameInstance` MyGameInstance))
  (set `local.Ref_WMasterInGame` (`/Game/Game/MyGameInstance.Ref_WidgetMasterInGame` _output_get))
  (set `local.Ref_Inventory` (`/Game/Game/MyGameInstance.Ref_Inventory` _output_get))
  (`|ExecutionSequence`
    (:`then_0`
      (set `local.Ref_ItemInfo` (`/Game/Game/Widget/W_MasterInGame.W_InventoryItemInfo` (`local.Ref_WMasterInGame`)))
      (set `local.ItemInfoOrCraft` true)
      (for _index (range 3)
        (set `local.IndexLoop` _index)
        (for _index_2 (range (+ (select `int` (`local.IndexLoop`) :`0` 6 :`1` 6 :`2` 7) 1))
          (set `local.IndexLoop1` _index_2)
          (bind _returnvalue (`|CreateWidget` "/Game/Game/Widget/Inventory/W_InventoryItemInfoSingleStat.W_InventoryItemInfoSingleStat_C"))
          (set `local.Ref_ItemInfoSingleStat` _returnvalue)
          (if (`local.ItemInfoOrCraft`)
            (`KismetArrayLibrary.Array_Add` (select `int` (`local.IndexLoop`) :`0` (`local.Ref_ItemInfo_NameAndRequrmest`) :`1` (`local.Ref_ItemInfo_MainStat`) :`2` (`local.Ref_ItemInfo_SecondStat`)) (`local.Ref_ItemInfoSingleStat`))
            (else
              (`KismetArrayLibrary.Array_Add` (select `int` (`local.IndexLoop`) :`0` (`local.Ref_Craft_ItemInfo_NameAndRequrmest`) :`1` (`local.Ref_Craft_ItemInfo_MainStat`) :`2` (`local.Ref_Craft_ItemInfo_SecondStat`)) (`local.Ref_ItemInfoSingleStat`))))
          (switch `int` (`local.IndexLoop`)
            (:`0`
              (`PanelWidget.AddChild` (`/Game/Game/Widget/Inventory/W_InventoryItemInfo.HorizontalBox_Requirements` (`local.Ref_ItemInfo`)) (`local.Ref_ItemInfoSingleStat`))
              (`TextBlock.SetColorAndOpacity` _textblock_statname (make `SlateColor` (struct :`R` 1.0 :`G` 1.0 :`B` 1.0 :`A` 1.0)))
              (`TextBlock.SetFont` _textblock_statname (make `SlateFontInfo` _font_fontobject _font_fontmaterial _font_outlinesettings "Bold" 10))
              (`TextBlock.SetText` _textblock_statname (`KismetTextLibrary.Conv_IntToText` (`local.IndexLoop1`)))
              (`TextBlock.SetFont` _textblock_statvalue (make `SlateFontInfo` _font_fontobject_3 _font_fontmaterial_3 _font_outlinesettings_3 "Regular" 10)))
            (:`1`
              (`PanelWidget.AddChild` (`/Game/Game/Widget/Inventory/W_InventoryItemInfo.VerticalBox_MainStat` (`local.Ref_ItemInfo`)) (`local.Ref_ItemInfoSingleStat`))
              (if (== (`local.IndexLoop1`) 0)
                (`TextBlock.SetFont` _textblock_statname_2 (make `SlateFontInfo` _font_fontobject_2 _font_fontmaterial_2 _font_outlinesettings_2 _font_typefacefontname 14))
                (`TextBlock.SetFont` _textblock_statvalue_2 (make `SlateFontInfo` _font_fontobject_4 _font_fontmaterial_4 _font_outlinesettings_4 _font_typefacefontname_2 14))))
            (:`2`
              (`PanelWidget.AddChild` (`/Game/Game/Widget/Inventory/W_InventoryItemInfo.VerticalBox_SecondStat` (`local.Ref_ItemInfo`)) (`local.Ref_ItemInfoSingleStat`)))))))
    (:`then_2`
      ;[1 1 1] End -- Set
      (set `/Game/Game/Inventory/Bp_Inventory.Ref_Widget_ItemInfo` (make `/Game/Game/Inventory/S_RefItemInfo` (`local.Ref_ItemInfo_NameAndRequrmest`) (`local.Ref_ItemInfo_MainStat`) (`local.Ref_ItemInfo_SecondStat`)) (`local.Ref_Inventory`))
      (set `/Game/Game/Inventory/Bp_Inventory.Ref_Widget_CraftItemInfoItem` (make `/Game/Game/Inventory/S_RefItemInfo` (`local.Ref_Craft_ItemInfo_NameAndRequrmest`) (`local.Ref_Craft_ItemInfo_MainStat`) (`local.Ref_Craft_ItemInfo_SecondStat`)) (`local.Ref_Inventory`)))))